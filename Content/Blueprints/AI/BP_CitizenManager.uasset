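; Citizen manager that tops up the population of AI characters in the game and provides events to spawn citizens and waypoints.
; A looping timer counts live BP_AI_Character actors and, while below the maximum, calls FindNextStreet on a random building from the player pawn's BP_Built_Manager.
; SpawnCitizen and SpawnWaypoint create actors at a supplied location but are not called within this graph.
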(event Custom|CheckSpawnedAICount
  (bind _builtmanagerref (Variables|Default|GetBuiltManagerRef))
  (bind _buildingsarray (Variables|/Game/Blueprints/Character/BP_Built_Manager.BP_Built_Manager_C|GetBuildingsArray _builtmanagerref))
  (bind _returnvalue (Utilities|Array|Length _buildingsarray))
  ;[1 1 1] Checks every 10 seconds how many Ai Character are in the Game and spawns new if Ai-Count < MaxSpawnedCitizen
  (bind _outactors (Actor|GetAllActorsOfClass "/Game/Blueprints/AI/BP_AI_Character.BP_AI_Character_C"))
  (Variables|Default|SetCitizenArray _outactors)
  (if (< (Utilities|Array|Length (Variables|Default|GetCitizenArray)) (Variables|Default|GetMaxSpawnedCitizen))
    (if (> _returnvalue 0)
      (Default|FindNextStreet (Utilities|Array|Get(acopy) _buildingsarray (Math|Random|RandomInteger _returnvalue))))))

(event Custom|SpawnCitizen
  (params (SpawnLocation :type Vector))
  (Game|SpawnActorfromClass "/Game/Blueprints/AI/BP_AI_Character.BP_AI_Character_C" (Math|Transform|MakeTransform SpawnLocation "0, 0, 0" "1,1,1") "Undefined" 0 0)
  (Variables|Default|SetCurrentlySpawnedCitizen (Utilities|Array|Length (Variables|Default|GetCitizenArray))))

(event Custom|SpawnWaypoint
  (params (SpawnLocation :type Vector))
  (Game|SpawnActorfromClass "/Game/Blueprints/AI/BP_Waypoints.BP_Waypoints_C" (Math|Transform|MakeTransform SpawnLocation "0, 0, 0" "1,1,1") "Undefined" 0 0))

(event EventBeginPlay
  (Utilities|FlowControl|Delay 1.0)
  (bind _asbp_built_manager (Utilities|Casting|CastToBP_Built_Manager (Game|Player|GetPlayerPawn 0)))
  (Variables|Default|SetBuiltManagerRef _asbp_built_manager)
  (Utilities|Time|SetTimerbyEvent (delegate Custom|CheckSpawnedAICount) 1e+01 true))

(fn ConstructionScript)