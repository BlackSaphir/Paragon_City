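; Shopping building child Blueprint that sets itself up in the city when it begins play.
; It caches the citizen manager and adds itself to the buildings array of the built manager, which is the player pawn.
; A timeline animates a material dissolve on the building mesh, then swaps in the final banner and shopping materials.
; It also calls FindNextStreet, presumably inherited, without waiting for the dissolve to finish.
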(event EventBeginPlay
  (bind _building_01 (Variables|Default|GetBuilding_01))
  (Utilities|FlowControl|Sequence
    (:then_0
      (bind _outactors (Actor|GetAllActorsOfClass "/Game/Blueprints/AI/BP_CitizenManager.BP_CitizenManager_C"))
      (Variables|Default|SetCitizenManagerRef (Utilities|Array|Get(acopy) _outactors))
      (bind _asbp_built_manager (Utilities|Casting|CastToBP_Built_Manager (Game|Player|GetPlayerPawn 0)))
      (bind _output_get (Variables|Default|SetBuiltManagerRef _asbp_built_manager))
      (Utilities|Array|Add (Variables|/Game/Blueprints/Character/BP_Built_Manager.BP_Built_Manager_C|GetBuildingsArray _output_get) self))
    (:then_1
      (Rendering|Material|SetScalarParameterValueonMaterials _building_01 "Texture Fade" 23.0))
    (:then_2
      (bind _newtrack_0 (Timeline|Timeline_1 PlayFromStart)
        (:Update
          (Rendering|Material|SetScalarParameterValueonMaterials _building_01 "Dissolve Amount" _newtrack_0))
        (:Finished
          (Rendering|Material|SetMaterial _building_01 0 "/Game/New_Assets/Materials/Instances/M_Banners_Inst.M_Banners_Inst")
          (Rendering|Material|SetMaterial _building_01 1 "/Game/New_Assets/Materials/Instances/M_Shopping.M_Shopping"))))
    (:then_3
      (CallFunction|FindNextStreet))))

(event Collision|EventActorBeginOverlap
  (params (OtherActor :type Actor%20Object%20Reference)))

(event EventTick
  (params (DeltaSeconds :type Float%20%28single-precision%29)))

(fn ConstructionScript
  (|CallParentFunction))