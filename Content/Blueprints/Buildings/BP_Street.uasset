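; Grid street tile for a building system that registers with BP_Built_Manager on BeginPlay and picks its mesh from adjacent streets.
; CheckKindOfStreet scans all BP_Street actors for exact 50-unit offsets, setting neighbour flags that select and rotate curve, T-junction or crossroad meshes.
; The construction script rotates Y-axis neighbours to line up.
; Overlap boxes report buildings in range or on the street to the manager, and clicks mark the tile selected.
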(event OnComponentBeginOverlap(LeftRangeBox)
  (params (OverlappedComponent :type Primitive%20Component%20Object%20Reference) (OtherActor :type Actor%20Object%20Reference) (OtherComp :type Primitive%20Component%20Object%20Reference) (OtherBodyIndex :type Integer) (bFromSweep :type Boolean) (SweepResult :type Hit%20Result%20Structure%20%28by%20ref%29))
  (if (Actor|ActorHasTag OtherActor "Building")
    (Variables|/Game/Blueprints/Character/BP_Built_Manager.BP_Built_Manager_C|SetbStreetInRange (Variables|Default|GetBuiltManagerRef) true)))

(event OnComponentEndOverlap(LeftRangeBox)
  (params (OverlappedComponent :type Primitive%20Component%20Object%20Reference) (OtherActor :type Actor%20Object%20Reference) (OtherComp :type Primitive%20Component%20Object%20Reference) (OtherBodyIndex :type Integer))
  (if (Actor|ActorHasTag OtherActor "Building")
    (Variables|/Game/Blueprints/Character/BP_Built_Manager.BP_Built_Manager_C|SetbStreetInRange (Variables|Default|GetBuiltManagerRef) false)))

(event OnComponentBeginOverlap(StreetBox)
  (params (OverlappedComponent :type Primitive%20Component%20Object%20Reference) (OtherActor :type Actor%20Object%20Reference) (OtherComp :type Primitive%20Component%20Object%20Reference) (OtherBodyIndex :type Integer) (bFromSweep :type Boolean) (SweepResult :type Hit%20Result%20Structure%20%28by%20ref%29))
  (if (Actor|ActorHasTag OtherActor "Building")
    (Variables|/Game/Blueprints/Character/BP_Built_Manager.BP_Built_Manager_C|SetbIsOnStreet (Variables|Default|GetBuiltManagerRef) true)))

(event OnComponentEndOverlap(StreetBox)
  (params (OverlappedComponent :type Primitive%20Component%20Object%20Reference) (OtherActor :type Actor%20Object%20Reference) (OtherComp :type Primitive%20Component%20Object%20Reference) (OtherBodyIndex :type Integer))
  (if (Actor|ActorHasTag OtherActor "Building")
    (Variables|/Game/Blueprints/Character/BP_Built_Manager.BP_Built_Manager_C|SetbIsOnStreet (Variables|Default|GetBuiltManagerRef) false)))

(event OnComponentBeginOverlap(RightRangeBox)
  (params (OverlappedComponent :type Primitive%20Component%20Object%20Reference) (OtherActor :type Actor%20Object%20Reference) (OtherComp :type Primitive%20Component%20Object%20Reference) (OtherBodyIndex :type Integer) (bFromSweep :type Boolean) (SweepResult :type Hit%20Result%20Structure%20%28by%20ref%29))
  (if (Actor|ActorHasTag OtherActor "Building")
    (Variables|/Game/Blueprints/Character/BP_Built_Manager.BP_Built_Manager_C|SetbStreetInRange (Variables|Default|GetBuiltManagerRef) true)))

(event OnComponentEndOverlap(RightRangeBox)
  (params (OverlappedComponent :type Primitive%20Component%20Object%20Reference) (OtherActor :type Actor%20Object%20Reference) (OtherComp :type Primitive%20Component%20Object%20Reference) (OtherBodyIndex :type Integer))
  (if (Actor|ActorHasTag OtherActor "Building")
    (Variables|/Game/Blueprints/Character/BP_Built_Manager.BP_Built_Manager_C|SetbStreetInRange (Variables|Default|GetBuiltManagerRef) false)))

(event OnClicked(Cube)
  (params (TouchedComponent :type Primitive%20Component%20Object%20Reference) (ButtonPressed :type Key%20Structure))
  (Variables|Default|SetStreetSelected true))

(event Custom|CheckKindOfStreet
  ;[1 1 1] Checks wich kind of street should be placed
  (bind _outactors (Actor|GetAllActorsOfClass "BP_Street_C"))
  (for _array_element _outactors
    (CallFunction|CheckforNeighbours _array_element)
    (CallFunction|CheckforCurves)))

(event EventBeginPlay
  (bind _asbp_built_manager (Utilities|Casting|CastToBP_Built_Manager (Game|Player|GetPlayerPawn 0)))
  (Variables|Default|SetBuiltManagerRef _asbp_built_manager)
  (Utilities|Array|Add (Variables|/Game/Blueprints/Character/BP_Built_Manager.BP_Built_Manager_C|GetStreetArr (Variables|Default|GetBuiltManagerRef)) self)
  (Utilities|Array|Add (Variables|/Game/Blueprints/Character/BP_Built_Manager.BP_Built_Manager_C|GetTempStreetArr (Variables|Default|GetBuiltManagerRef)) self))

(fn ConstructionScript
  (bind _cube (Variables|Default|GetCube))
  (bind _returnvalue (Transformation|GetWorldLocation _cube))
  (bind _outactors (Actor|GetAllActorsOfClass "BP_Street_C"))
  (for _array_element _outactors
    (if (and (or (== (.y (Transformation|GetWorldLocation (Variables|BP_Street_C|GetCube _array_element))) (- (.y _returnvalue) 5e+01)) (== (.y (Transformation|GetWorldLocation (Variables|BP_Street_C|GetCube _array_element))) (+ (.y _returnvalue) 5e+01))) (== (.x (Transformation|GetWorldLocation (Variables|BP_Street_C|GetCube _array_element))) (.x _returnvalue)))
      (bind _output_get (Variables|Default|SetrightNeighbour true))
      (bind _output_get_2 (Variables|Default|SetleftNeighbour true))
      (if (or _output_get _output_get_2)
        (Transformation|SetWorldRotation (Variables|BP_Street_C|GetCube _array_element) "0,90.000000, 0" false false)
        (Transformation|SetWorldRotation (Variables|Default|GetCube) "0,90.000000, 0" false false)
        (Variables|Default|SetleftNeighbour false)
        (Variables|Default|SetrightNeighbour false)))))

(fn CheckforCurves
  (Utilities|FlowControl|Sequence
    (:then_0
      ;[1 1 1] Buttom Left -> Top
      (if (Math|Boolean|ANDBoolean (Variables|Default|GetleftNeighbour) (not (Variables|Default|GetrightNeighbour)) (Variables|Default|GetaboveNeighbour) (not (Variables|Default|GetbelowNeighbour)))
        (Components|StaticMesh|SetStaticMesh (Variables|Default|GetCube) "/Game/Meshes/Street/Streets_Test_StreetModule_3.Streets_Test_StreetModule_3")
        (Transformation|SetWorldRotation (Variables|Default|GetCube) "0, 0, 0" false false)))
    (:then_1
      ;[1 1 1] Top Left -> Buttom
      (if (Math|Boolean|ANDBoolean (Variables|Default|GetleftNeighbour) (not (Variables|Default|GetrightNeighbour)) (not (Variables|Default|GetaboveNeighbour)) (Variables|Default|GetbelowNeighbour))
        (Components|StaticMesh|SetStaticMesh (Variables|Default|GetCube) "/Game/Meshes/Street/Streets_Test_StreetModule_3.Streets_Test_StreetModule_3")
        (Transformation|SetWorldRotation (Variables|Default|GetCube) "0,-90.000000, 0" false false)))
    (:then_2
      ;[1 1 1] Top Right -> Buttom
      (if (Math|Boolean|ANDBoolean (not (Variables|Default|GetleftNeighbour)) (Variables|Default|GetrightNeighbour) (not (Variables|Default|GetaboveNeighbour)) (Variables|Default|GetbelowNeighbour))
        (Components|StaticMesh|SetStaticMesh (Variables|Default|GetCube) "/Game/Meshes/Street/Streets_Test_StreetModule_3.Streets_Test_StreetModule_3")
        (Transformation|SetWorldRotation (Variables|Default|GetCube) "0,180.000000, 0" false false)))
    (:then_3
      ;[1 1 1] Buttom Right -> Top
      (if (Math|Boolean|ANDBoolean (not (Variables|Default|GetleftNeighbour)) (Variables|Default|GetrightNeighbour) (Variables|Default|GetaboveNeighbour) (not (Variables|Default|GetbelowNeighbour)))
        (Components|StaticMesh|SetStaticMesh (Variables|Default|GetCube) "/Game/Meshes/Street/Streets_Test_StreetModule_3.Streets_Test_StreetModule_3")
        (Transformation|SetWorldRotation (Variables|Default|GetCube) "0,90.000000, 0" false false)))))

(fn CheckforNeighbours
  (params (Neighbour :type BP%20Street%20Object%20Reference))
  (bind _cube (Variables|BP_Street_C|GetCube Neighbour))
  (bind _cube_2 (Variables|Default|GetCube))
  (bind _cube_3 (Variables|BP_Street_C|GetCube Neighbour))
  (bind _cube_4 (Variables|Default|GetCube))
  (bind _cube_5 (Variables|BP_Street_C|GetCube Neighbour))
  (bind _cube_6 (Variables|Default|GetCube))
  (bind _cube_7 (Variables|BP_Street_C|GetCube Neighbour))
  (bind _cube_8 (Variables|Default|GetCube))
  (bind _returnvalue (Transformation|GetWorldLocation _cube_7))
  (bind _returnvalue_2 (Transformation|GetWorldLocation _cube_8))
  (bind _returnvalue_3 (Transformation|GetWorldLocation _cube))
  (bind _returnvalue_4 (Transformation|GetWorldLocation _cube_2))
  (bind _returnvalue_5 (Transformation|GetWorldLocation _cube_3))
  (bind _returnvalue_6 (Transformation|GetWorldLocation _cube_4))
  (bind _returnvalue_7 (Transformation|GetWorldLocation _cube_5))
  (bind _returnvalue_8 (Transformation|GetWorldLocation _cube_6))
  ;[1 1 1] Check Neighbours
  (Utilities|FlowControl|Sequence
    (:then_0
      (if (and (and (== (.x _returnvalue_3) (.x _returnvalue_4)) (== (.y _returnvalue_3) (- (.y _returnvalue_4) 5e+01))) (not (Utilities|Array|ContainsItem (Variables|Default|GetCrossNeighArr) Neighbour)))
        (Variables|Default|SetleftNeighbour true)
        ;[1 1 1] Jump to Check for Crossroads
        (CallFunction|CheckforCrossroads :!label _label)))
    (:then_1
      (if (and (and (== (.x _returnvalue_7) (.x _returnvalue_8)) (== (.y _returnvalue_7) (+ (.y _returnvalue_8) 5e+01))) (not (Utilities|Array|ContainsItem (Variables|Default|GetCrossNeighArr) Neighbour)))
        (Variables|Default|SetrightNeighbour true)
        (goto _label)))
    (:then_2
      (if (and (and (== (.x _returnvalue) (+ (.x _returnvalue_2) 5e+01)) (== (.y _returnvalue) (.y _returnvalue_2))) (not (Utilities|Array|ContainsItem (Variables|Default|GetCrossNeighArr) Neighbour)))
        (Variables|Default|SetaboveNeighbour true)
        (goto _label)))
    (:then_3
      (if (and (and (== (.x _returnvalue_5) (- (.x _returnvalue_6) 5e+01)) (== (.y _returnvalue_5) (.y _returnvalue_6))) (not (Utilities|Array|ContainsItem (Variables|Default|GetCrossNeighArr) Neighbour)))
        (Variables|Default|SetbelowNeighbour true)
        (goto _label)))))

(fn CheckforCrossroads
  ;[1 1 1] Top open
  (if (Math|Boolean|ANDBoolean (Variables|Default|GetleftNeighbour) (Variables|Default|GetrightNeighbour) (Variables|Default|GetaboveNeighbour) (not (Variables|Default|GetbelowNeighbour)))
    (Components|StaticMesh|SetStaticMesh (Variables|Default|GetCube) "/Game/Meshes/Street/Streets_Test_StreetModule_4.Streets_Test_StreetModule_4")
    (Transformation|SetWorldRotation (Variables|Default|GetCube) "0,90.000000, 0" false false)
    (else
      ;[1 1 1] Buttom open
      (if (Math|Boolean|ANDBoolean (Variables|Default|GetleftNeighbour) (Variables|Default|GetrightNeighbour) (not (Variables|Default|GetaboveNeighbour)) (Variables|Default|GetbelowNeighbour))
        (Components|StaticMesh|SetStaticMesh (Variables|Default|GetCube) "/Game/Meshes/Street/Streets_Test_StreetModule_4.Streets_Test_StreetModule_4")
        (Transformation|SetWorldRotation (Variables|Default|GetCube) "0,-90.000000, 0" false false)
        (else
          ;[1 1 1] Left open
          (if (Math|Boolean|ANDBoolean (Variables|Default|GetleftNeighbour) (not (Variables|Default|GetrightNeighbour)) (Variables|Default|GetaboveNeighbour) (Variables|Default|GetbelowNeighbour))
            (Components|StaticMesh|SetStaticMesh (Variables|Default|GetCube) "/Game/Meshes/Street/Streets_Test_StreetModule_4.Streets_Test_StreetModule_4")
            (Transformation|SetWorldRotation (Variables|Default|GetCube) "0, 0, 0" false false)
            (else
              ;[1 1 1] Right open
              (if (Math|Boolean|ANDBoolean (not (Variables|Default|GetleftNeighbour)) (Variables|Default|GetrightNeighbour) (Variables|Default|GetaboveNeighbour) (Variables|Default|GetbelowNeighbour))
                (Components|StaticMesh|SetStaticMesh (Variables|Default|GetCube) "/Game/Meshes/Street/Streets_Test_StreetModule_4.Streets_Test_StreetModule_4")
                (Transformation|SetWorldRotation (Variables|Default|GetCube) "0,180.000000, 0" false false)
                (else
                  ;[1 1 1] Full Crossroad
                  (if (Math|Boolean|ANDBoolean (Variables|Default|GetleftNeighbour) (Variables|Default|GetrightNeighbour) (Variables|Default|GetaboveNeighbour) (Variables|Default|GetbelowNeighbour))
                    (Components|StaticMesh|SetStaticMesh (Variables|Default|GetCube) "/Game/Meshes/Street/Streets_Test_StreetModule_1.Streets_Test_StreetModule_1")))))))))))